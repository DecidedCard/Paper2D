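; BP_Monster is an enemy that finds a BP_Knight, chases it and attacks when close.
; Tick runs UpdateAI, a state switch where Idle acquires the knight as TargetEnemy and enters Move.
; Move calls BeginAttack within a fixed range, otherwise sets a four-way Direction from the dominant X or Z axis toward the target.
; Movement and attack logic are not implemented in these graphs.
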(event `self.ReceiveBeginPlay`
  (`parent.ReceiveBeginPlay`))

(event `self.ReceiveTick`
  (params (DeltaSeconds :type "Float (single-precision)"))
  (`parent.ReceiveTick` DeltaSeconds)
  (`self.UpdateAI`))

(fn `UpdateAI`
  (bind _targetenemy (`self.TargetEnemy`))
  (bind (_chasedirection_x _chasedirection_y _chasedirection_z) (`KismetMathLibrary.BreakVector` (`self.ChaseDirection`)))
  (switch `/Game/Blueprints/EState` (`self.State`)
    (:`NewEnumerator0`
      (bind _returnvalue (`GameplayStatics.GetActorOfClass` "/Game/Blueprints/BP_Knight.BP_Knight_C"))
      (bind _output_get (set `self.TargetEnemy` _returnvalue))
      (`/Engine/EditorBlueprintResources/StandardMacros.IsValid` _output_get
        (:`Is Valid`
          (set `self.State` "NewEnumerator1"))))
    (:`NewEnumerator1`
      (`/Engine/EditorBlueprintResources/StandardMacros.IsValid` _targetenemy
        (:`Is Valid`
          (bind _output_get_2 (set `self.ChaseDirection` (- (`self.K2_GetActorLocation` _targetenemy) (`self.K2_GetActorLocation`))))
          (if (< (`KismetMathLibrary.VSize` _output_get_2) 300.0)
            (`self.BeginAttack`)
            (elif (> (`KismetMathLibrary.Abs` _chasedirection_x) (`KismetMathLibrary.Abs` _chasedirection_z))
              (`/Engine/EditorBlueprintResources/StandardMacros.CompareFloat` _chasedirection_x
                (:`>`
                  (set `self.Direction` "NewEnumerator3"))
                (:`<`
                  (set `self.Direction` "NewEnumerator2")))
              (else
                (`/Engine/EditorBlueprintResources/StandardMacros.CompareFloat` _chasedirection_z
                  (:`>`
                    (set `self.Direction` "NewEnumerator0"))
                  (:`<`
                    (set `self.Direction` "NewEnumerator1")))))))))))

(fn `UserConstructionScript`
  (`parent.UserConstructionScript`))