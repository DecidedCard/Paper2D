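; Player controller that turns movement input into state and facing for the controlled BP_Knight, which it caches on BeginPlay.
; Each Tick, UpdateInput switches the knight between Idle and Move, holding Move while input is active or its destination is not yet reached.
; It also sets one of four directions, with horizontal input overriding vertical, and raises StopMove when both axes are zero.
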(event `self.ReceiveBeginPlay`
  (bind _asbp_knight (cast `/Game/Blueprints/Creatures/BP_Knight` (`self.K2_GetPawn`)))
  (set `self.MyPlayer` _asbp_knight))

(event `self.ReceiveTick`
  (params (DeltaSeconds :type "Float (single-precision)"))
  (`self.UpdateInput`))

(fn `UpdateInput`
  (bind _myplayer (`self.MyPlayer`))
  (switch `/Game/Blueprints/Struct/EState` (`/Game/Blueprints/Creatures/BP_Creature.State` (`self.MyPlayer`))
    (:`NewEnumerator0`
      _)
    (:`NewEnumerator1`
      _))
  (`|ExecutionSequence`
    (:`then_0`
      (if (or (!= (`self.GetInputAxisValue`) 0.0) (!= (`self.GetInputAxisValue`) 0.0) (not (`/Game/Blueprints/Creatures/BP_Creature.HasArrivedToDest` (`self.MyPlayer`))))
        (set `/Game/Blueprints/Creatures/BP_Creature.State` "NewEnumerator1" _myplayer)
        (else
          (set `/Game/Blueprints/Creatures/BP_Creature.State` "NewEnumerator0" _myplayer))))
    (:`then_1`
      (`/Engine/EditorBlueprintResources/StandardMacros.CompareFloat` (`self.GetInputAxisValue`)
        (:`>`
          (set `/Game/Blueprints/Creatures/BP_Creature.Direction` "NewEnumerator0" _myplayer))
        (:`<`
          (set `/Game/Blueprints/Creatures/BP_Creature.Direction` "NewEnumerator1" _myplayer))))
    (:`then_2`
      (`/Engine/EditorBlueprintResources/StandardMacros.CompareFloat` (`self.GetInputAxisValue`)
        (:`>`
          (set `/Game/Blueprints/Creatures/BP_Creature.Direction` "NewEnumerator3" _myplayer))
        (:`<`
          (set `/Game/Blueprints/Creatures/BP_Creature.Direction` "NewEnumerator2" _myplayer))))
    (:`then_3`
      (set `/Game/Blueprints/Creatures/BP_Creature.bStopMove` (and (== (`self.GetInputAxisValue`) 0.0) (== (`self.GetInputAxisValue`) 0.0)) (`self.MyPlayer`)))))

(fn `UserConstructionScript`)